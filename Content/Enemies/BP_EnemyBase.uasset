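; BP_EnemyBase is a base enemy that flies along its spawn-time forward vector and fires on a timer.
; Tick moves it without sweep and spawns Ammo at FirePoint, matching its rotation, whenever the shot delay elapses.
; Overlapping a Player-tagged actor calls OnEnemyDestroy and notifies BP_SS_GameMode; the bound handler destroys the enemy after a brief delay.
; An ammo-overlap cast leading to the same destroy path is left unconnected.
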(event Custom|Destroyed_Event
  ;[1 1 1] Move Input
  (Utilities|FlowControl|Delay 0.1)
  (Actor|DestroyActor))

(event EventBeginPlay
  ;[1 1 1] Move Input
  (Variables|Default|SetMovementVector (Transformation|GetActorForwardVector))
  (EventDispatchers|BindEventtoOnEnemyDestroy (delegate Custom|Destroyed_Event)))

(event Collision|EventActorBeginOverlap
  (params (OtherActor :type Actor%20Object%20Reference))
  ;[1 1 1] Collision Check
  (if (Utilities|Array|ContainsItem (Variables|/Script/Engine.Actor|GetTags OtherActor) "Player")
    (Default|CallOnEnemyDestroy)
    (bind _asbp_ss_game_mode (Utilities|Casting|CastToBP_SS_GameMode (Game|GetGameMode)))
    (Default|EnemyDestroyed _asbp_ss_game_mode)))

(event EventTick
  (params (DeltaSeconds :type Float%20%28single-precision%29))
  ;[1 1 1] MoveAndFire
  (CallFunction|Move DeltaSeconds)
  (bind _output_get (Variables|Default|SetShotCurrentTime (+ DeltaSeconds (Variables|Default|GetShotCurrentTime))))
  (if (> _output_get (Variables|Default|GetDelayShoot))
    (Variables|Default|SetShotCurrentTime 0.0)
    (CallFunction|Fire)))

(fn ConstructionScript)

(fn Move
  (params (DeltaTime :type Float%20%28double-precision%29))
  (Transformation|SetActorLocation (+ (Transformation|GetActorLocation) (* (* DeltaTime (Variables|Default|GetSpeed)) (Variables|Default|GetMovementVector))) false false))

(fn Fire
  (bind _returnvalue (Game|SpawnActorfromClass (Variables|Default|GetAmmo) (Transformation|GetWorldTransform (Variables|Default|GetFirePoint)) "Undefined" "MultiplyWithRoot" 0 0))
  (Transformation|SetActorRotation _returnvalue (Transformation|GetActorRotation)))